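; BP_Plane_Pawn is a player-controlled plane pawn that constantly moves forward along the direction it faces.
; Tick counter-rotates the left and right propellers at a shared speed variable and feeds the actor's forward vector into AddMovementInput.
; The roll and pitch input axes rotate the whole actor locally at a fixed, frame-time-scaled rate, thereby steering the flight.
; A body-roll node is left disconnected, and NewFunction_0 is empty.
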(event `self.ReceiveTick`
  (params (DeltaSeconds :type "Float (single-precision)"))
  (set `self.Delta Seconds_0` DeltaSeconds)
  (`|ExecutionSequence`
    (:`then_0`
      ;[1 1 1] 왼쪽 프로펠러 회전
      (`SceneComponent.K2_AddLocalRotation` (`self.left_0`) (`KismetMathLibrary.MakeRotator` (* (`GameplayStatics.GetWorldDeltaSeconds`) (`self.PropellerRotateSpeed_0`))) false false)
      (`KismetSystemLibrary.Delay` 1.0))
    (:`then_1`
      ;[1 1 1] 오른쪽 프로펠러 회전
      (`SceneComponent.K2_AddLocalRotation` (`self.right_0`) (`KismetMathLibrary.MakeRotator` (* (`GameplayStatics.GetWorldDeltaSeconds`) (`self.PropellerRotateSpeed_0`) -1.0)) false false))
    (:`then_2`
      ;[1 1 1] 비행기 이동
      (`self.AddMovementInput` (`self.GetActorForwardVector`)))))

(event `InputAxis|roll`
  (params (AxisValue :type "Float (single-precision)"))
  ;[1 1 1] 롤 회전
  (`self.K2_AddActorLocalRotation` (`KismetMathLibrary.MakeRotator` (* AxisValue 60.0 (`GameplayStatics.GetWorldDeltaSeconds`)))))

(event `InputAxis|pitch`
  (params (AxisValue :type "Float (single-precision)"))
  ;[1 1 1] 피치 회전
  (`self.K2_AddActorLocalRotation` (`KismetMathLibrary.MakeRotator` 0.0 (* AxisValue 60.0 (`GameplayStatics.GetWorldDeltaSeconds`)))))

(fn `NewFunction_0`)

(fn `UserConstructionScript`)